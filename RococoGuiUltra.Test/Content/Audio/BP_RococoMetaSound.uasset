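; BP_RococoMetaSound wraps a persistent 2D audio stream, created from its Sound on BeginPlay, behind a volume control.
; SetVolume stores a new value and calls OnVolumeChanged only when the volume differs.
; OnVolumeChanged pauses the stream at or below MinVolume, otherwise applies the multiplier, unpauses and starts playback if needed.
; Auto-destroy is off so the component stays reusable, and persistence across level transitions is configurable.
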(event `self.ReceiveBeginPlay`
  (bind _returnvalue (`GameplayStatics.CreateSound2D` (`self.Sound`) 1.0 1.0 0.0 null (`self.PersistAcrossLevelTransition`) false))
  (set `self.AudioStream` _returnvalue))

(fn `OnVolumeChanged`
  (bind _audiostream (`self.AudioStream`))
  (`/Engine/EditorBlueprintResources/StandardMacros.IsValid` (`self.AudioStream`)
    (:`Is Valid`
      (if (<= (`self.Volume`) (`self.MinVolume`))
        (`AudioComponent.SetPaused` _audiostream true)
        (else
          (`AudioComponent.SetVolumeMultiplier` _audiostream (`self.Volume`))
          (`AudioComponent.SetPaused` (`self.AudioStream`) false)
          (if (not (`AudioComponent.IsPlaying` (`self.AudioStream`)))
            (`AudioComponent.Play` (`self.AudioStream`) 0.0)))))))

(fn `SetVolume`
  (params (Volume :type "Float (double-precision)"))
  (if (not (== Volume (`self.Volume`)))
    (set `self.Volume` Volume)
    (`self.OnVolumeChanged`)))